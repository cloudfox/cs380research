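; BP_SquadManager is a squad manager actor that spawns a group of BP_Agent actors around itself when play begins.
; For each slot in its Agents array, it spawns an agent at a random horizontal offset within a fixed radius, using the manager's rotation and scale.
; Each new agent receives a reference back to the manager and is written into its array slot, so the array's length determines squad size.
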(event EventBeginPlay
  (bind _returnvalue (Transformation|GetActorTransform))
  (bind _returnvalue_2 (Math|Random|RandomUnitVector))
  (Utilities|FlowControl|Sequence
    (:then_0
      (for (_ _array_index) (Variables|Default|Getagents)
        (bind _returnvalue_3 (Game|SpawnActorfromClass "/Game/Blueprints/BP_Agent.BP_Agent_C" (Math|Transform|MakeTransform (+ (.location _returnvalue) (* (Math|Vector|MakeVector (.x _returnvalue_2) (.y _returnvalue_2) 0.0) 2.5e+02)) (.rotation _returnvalue) (.scale _returnvalue)) "Undefined" 0 0))
        (Variables|/Script/cs380researchproject.Agent|SetSquadManager _returnvalue_3 self)
        (Utilities|Array|SetArrayElem (Variables|Default|Getagents) _array_index _returnvalue_3)))))

(fn ConstructionScript)