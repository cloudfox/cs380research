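; BPC_SightNode is a search node that registers as found with its enclosing BP_SearchZone when sighted.
; Shortly after BeginPlay it disables collision on its Sphere, then queries that Sphere's overlaps to cache the parent zone.
; The sighted event, called from outside this graph, acts only once: it turns the sphere green, notifies the zone and latches NodeFound.
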(event Custom|sighted
  (if (not (Variables|Default|GetNodeFound))
    (Rendering|Material|SetMaterial (Variables|Default|GetSphere) 0 "/Game/Materials/M_Green.M_Green")
    (Default|NodeFound (Variables|Default|GetparentZone) self)
    (Variables|Default|SetNodeFound true)))

(event EventBeginPlay
  (Utilities|FlowControl|Delay 0.2)
  (Collision|SetCollisionEnabled (Variables|Default|GetSphere) "NoCollision")
  (for _array_element (Collision|GetOverlappingActors (Variables|Default|GetSphere) "/Game/Blueprints/BP_SearchZone.BP_SearchZone_C" :!class /Script/Engine.PrimitiveComponent)
    (bind _asbp_search_zone (Utilities|Casting|CastToBP_SearchZone _array_element))
    (Variables|Default|SetparentZone _asbp_search_zone)))

(fn ConstructionScript)