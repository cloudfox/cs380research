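; Search zone actor that tracks the sight nodes inside its box and displays how many remain to be found.
; Shortly after BeginPlay it registers each overlapping BPC_SightNode, setting itself as that node's parent zone.
; NodeFound removes a node from the list and updates the count on the text render.
; Grid-spawning logic for nodes is present but disconnected, and the construction script does nothing.
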(event Custom|NodeFound
  (params (node :type BPC%20Sight%20Node%20Object%20Reference))
  (Math|Integer|DecrementInt (Variables|Default|GetNodeCount)
    (:%20%20
      (Rendering|Components|TextRender|SetText (Variables|Default|GetTextRender) (Utilities|Text|ToText(Integer) (Variables|Default|GetNodeCount)))
      (Utilities|Array|RemoveItem (Variables|Default|GetSearchNodes) node))))

(event EventBeginPlay
  (Utilities|FlowControl|Delay 0.1)
  (for _array_element (Collision|GetOverlappingActors (Variables|Default|GetBox) "/Game/Blueprints/BPC_SightNode.BPC_SightNode_C" :!class /Script/Engine.PrimitiveComponent)
    (bind _asbpc_sight_node (Utilities|Casting|CastToBPC_SightNode _array_element))
    (Variables|/Game/Blueprints/BPC_SightNode.BPC_SightNode_C|SetparentZone _asbpc_sight_node self)
    (Math|Integer|IncrementInt (Variables|Default|GetNodeCount)
      (:%20%20
        (Utilities|Array|Add (Variables|Default|GetSearchNodes) _asbpc_sight_node))))
  (Rendering|Components|TextRender|SetText (Variables|Default|GetTextRender) (Utilities|Text|ToText(Integer) (Variables|Default|GetNodeCount))))

(fn ConstructionScript)